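; BP_BulletAttack is a hitscan attack actor that fires an instant bullet shot in a given look direction.
; UseAttack runs an object line trace from the actor's location out to MaxTravel against pawns, world static and dynamic objects, and physics bodies.
; If the hit actor has a BPC_Health component, it receives DamageAmount through TakeDamage.
; The trace draws a one-frame debug line.
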(event EventBeginPlay
  (|CallParentFunction) ; This node is disabled and will not be called.\nDrag off pins to build functionality.
)

(event Collision|EventActorBeginOverlap
  (params (OtherActor :type Actor%20Object%20Reference))
  (|CallParentFunction OtherActor) ; This node is disabled and will not be called.\nDrag off pins to build functionality.
)

(event EventTick
  (params (DeltaSeconds :type Float%20%28single-precision%29))
  (|CallParentFunction DeltaSeconds) ; This node is disabled and will not be called.\nDrag off pins to build functionality.
)

(event EventUseAttack
  (params (Look%20Direction :type Vector :default "0, 0, 0"))
  (bind _returnvalue (Transformation|GetActorLocation))
  (bind (_outhit _returnvalue_2) (Collision|LineTraceForObjects _returnvalue (+ _returnvalue (* Look%20Direction (Variables|Default|GetMax%20Travel))) (Utilities|Array|MakeArray "ObjectTypeQuery3" "ObjectTypeQuery1" "ObjectTypeQuery2" "ObjectTypeQuery4") false 0 "ForOneFrame"))
  (if _returnvalue_2
    (Utilities|IsValid (Actor|GetComponentbyClass (.HitActor (Collision|BreakHitResult _outhit)) "/Game/Components/BPC_Health.BPC_Health_C")
      (:Is%20Valid
        (Default|TakeDamage (Actor|GetComponentbyClass (.HitActor (Collision|BreakHitResult _outhit)) "/Game/Components/BPC_Health.BPC_Health_C") (Variables|Default|GetDamage%20Amount))))))

(fn ConstructionScript
  (|CallParentFunction))