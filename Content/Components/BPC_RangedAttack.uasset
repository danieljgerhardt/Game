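; Actor component that fires the owner's currently selected ranged attack.
; UseAttack gets the look direction from the owner, spawns the CurrentAttack class slightly ahead of and above it, then passes that direction to the spawned actor's own UseAttack.
; SetAttack swaps the attack class, and ResetCooldown re-enables CanCast and invalidates the cooldown timer handle, though UseAttack itself neither checks nor starts a cooldown.
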(event EventBeginPlay)

(event EventTick
  (params (DeltaSeconds :type Float%20%28single-precision%29)))

(fn UseAttack
  (bind _returnvalue (Components|GetOwner))
  (bind _look_direction (Class|BPICharacter|GetLookDirection(Message) _returnvalue))
  (bind _returnvalue_2 (Game|SpawnActorfromClass (Variables|Default|GetCurrent%20Attack) (Math|Conversions|ToTransform(Vector) (+ (* _look_direction 1e+02) (Transformation|GetActorLocation _returnvalue) "0.000000,0.000000,50.000000")) "Undefined" "MultiplyWithRoot" 0 0))
  (Utilities|IsValid _returnvalue_2
    (:Is%20Valid
      (Default|UseAttack _returnvalue_2 _look_direction))))

(fn SetAttack
  (params (Attack%20Class :type BP%20Base%20Attack%20Class%20Reference))
  (Variables|Default|SetCurrent%20Attack Attack%20Class))

(fn ResetCooldown
  (Variables|Default|SetCan%20Cast true)
  (Utilities|Time|InvalidateTimerHandle (Variables|Default|GetCooldown%20Timer)))