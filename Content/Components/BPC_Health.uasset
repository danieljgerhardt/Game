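; Health component that tracks an actor's current health, starting at max, with functions for damage and healing.
; Damage refreshes the health bar and calls DieMessage on the owner at zero or below, while healing adds health without clamping or refreshing.
; The bar update targets W_WorldHealthBar in the owner's widget components, or the first player's BP_PlayerHUD bar when the owner has no widget components.
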(event EventBeginPlay
  (Variables|Default|SetCurrent%20Health (Variables|Default|GetMax%20Health)))

(event EventTick
  (params (DeltaSeconds :type Float%20%28single-precision%29)))

(fn TakeDamage
  (params (Incoming%20Damage :type Float%20%28double-precision%29))
  (bind _output_get (Variables|Default|SetCurrent%20Health (- (Variables|Default|GetCurrent%20Health) Incoming%20Damage)))
  (CallFunction|UpdateHealthBar)
  (if (<= _output_get 0.0)
    (CallFunction|Die)))

(fn Heal
  (params (Heal%20Amount :type Float%20%28double-precision%29))
  (Variables|Default|SetCurrent%20Health (+ (Variables|Default|GetCurrent%20Health) Heal%20Amount)))

(fn Die
  (Class|BPICharacter|Die(Message) (Components|GetOwner)))

(fn UpdateHealthBar
  (bind _returnvalue (Components|GetOwner))
  (bind _returnvalue_2 (Actor|GetComponentsByClass _returnvalue "/Script/UMG.WidgetComponent"))
  (for _array_element _returnvalue_2
    ;[0.15 0.15 0.15 0.5] Logic For Enemies
    (bind _asw_world_health_bar (Utilities|Casting|CastToW_WorldHealthBar (UserInterface|GetWidget _array_element)))
    (Default|UpdateHealth _asw_world_health_bar (Variables|Default|GetCurrent%20Health) (Variables|Default|GetMax%20Health)))
  (if (== (Utilities|Array|Length _returnvalue_2) 0)
    (bind _asbp_player_hud (Utilities|Casting|CastToBP_PlayerHUD (HUD|GetHUD (Game|GetPlayerController (Game|GetPlayerState 0)))))
    (Default|UpdateHealth (Variables|/Game/UI/BP_PlayerHUD.BP_PlayerHUD_C|GetPlayer%20Health%20Bar _asbp_player_hud) (Variables|Default|GetCurrent%20Health) (Variables|Default|GetMax%20Health))))