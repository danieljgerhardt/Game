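; Actor component that tracks a mana pool for its owner, starting full at MaxMana on BeginPlay.
; Use Mana subtracts the given amount without any clamp or affordability check, so CurrentMana can go negative.
; Restore Mana adds the given amount and clamps the result between zero and MaxMana.
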(event EventBeginPlay
  (Variables|Default|SetCurrent%20Mana (Variables|Default|GetMax%20Mana)))

(event EventTick
  (params (DeltaSeconds :type Float%20%28single-precision%29)))

(fn UseMana
  (params (Mana%20Used :type Float%20%28double-precision%29))
  (Variables|Default|SetCurrent%20Mana (- (Variables|Default|GetCurrent%20Mana) Mana%20Used)))

(fn RestoreMana
  (params (Mana%20Restore :type Float%20%28double-precision%29))
  (Variables|Default|SetCurrent%20Mana (Math|Float|Clamp(Float) (+ (Variables|Default|GetCurrent%20Mana) Mana%20Restore) 0.0 (Variables|Default|GetMax%20Mana))))