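; BPC_SpellCasting is an actor component that lets its owner cast a swappable primary spell, defaulting to BP_Fireball on BeginPlay.
; CastPrimarySpell gets the owner's look direction through a message call and spawns the current spell class a short distance along it.
; If the spawn succeeds, it calls CastSpell on the new actor with that direction.
; SetPrimarySpell replaces the stored spell class.
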(event EventBeginPlay
  (Variables|Default|SetCurrent%20Primary%20Spell "/Game/Spells/BP_Fireball.BP_Fireball_C"))

(event EventTick
  (params (DeltaSeconds :type Float%20%28single-precision%29)))

(fn CastPrimarySpell
  (bind _returnvalue (Components|GetOwner))
  (bind _look_direction (Class|BPICharacter|GetLookDirection(Message) _returnvalue))
  (bind _returnvalue_2 (Game|SpawnActorfromClass (Variables|Default|GetCurrent%20Primary%20Spell) (Math|Conversions|ToTransform(Vector) (+ (Transformation|GetActorLocation _returnvalue) (* _look_direction 1e+02))) "Undefined" "MultiplyWithRoot" 0 0))
  (Utilities|IsValid _returnvalue_2
    (:Is%20Valid
      (Default|CastSpell _returnvalue_2 _look_direction))))

(fn SetPrimarySpell
  (params (Spell%20Class :type BP%20Base%20Spell%20Class%20Reference))
  (Variables|Default|SetCurrent%20Primary%20Spell Spell%20Class))