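; BPC_SpellCast is an actor component that lets its owner cast the currently selected spell.
; Cast Spell requires a charge and no active cooldown, spawns the spell actor at the owner's location, then passes it the owner's look direction.
; A successful cast empties all charges and starts a timer using the spell's own cooldown, which re-enables casting.
; Separate functions set the spell class and add charges.
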(event EventBeginPlay)

(event EventTick
  (params (DeltaSeconds :type Float%20%28single-precision%29)))

(fn CastSpell
  (bind _returnvalue (Components|GetOwner))
  (if (and (Variables|Default|GetCan%20Cast) (> (Variables|Default|GetSpell%20Charges) 0))
    (bind _look_direction (Class|BPICharacter|GetLookDirection(Message) _returnvalue))
    (bind _returnvalue_2 (Game|SpawnActorfromClass (Variables|Default|GetCurrent%20Spell) (Math|Conversions|ToTransform(Vector) (Transformation|GetActorLocation _returnvalue)) "Undefined" "MultiplyWithRoot" _returnvalue 0))
    (Utilities|IsValid _returnvalue_2
      (:Is%20Valid
        (if (not (Utilities|Time|IsValidTimerHandle (Variables|Default|GetCooldown%20Timer)))
          (Default|CastSpell _returnvalue_2 _look_direction)
          (bind _returnvalue_3 (Utilities|Time|SetTimerbyFunctionName 0 "Reset Cooldown" (Variables|/Game/Spells/SpellBlueprints/BP_BaseSpell.BP_BaseSpell_C|GetCooldown _returnvalue_2)))
          (Variables|Default|SetCooldown%20Timer _returnvalue_3)
          (Variables|Default|SetCan%20Cast false)
          (Variables|Default|SetSpell%20Charges 0))))))

(fn SetSpell
  (params (Spell%20Class :type BP%20Base%20Spell%20Class%20Reference))
  (Variables|Default|SetCurrent%20Spell Spell%20Class))

(fn ResetCooldown
  (Variables|Default|SetCan%20Cast true)
  (Utilities|Time|InvalidateTimerHandle (Variables|Default|GetCooldown%20Timer)))

(fn IncreaseSpellCharge
  (Math|Integer|IncrementInt (Variables|Default|GetSpell%20Charges)
    (:%20%20
      (return))))