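; BPC_MeleeAttack is an actor component that gives its owner a melee attack through the UseMeleeAttack function.
; It gets the look direction through a message to the owner, then sweeps a single capsule trace for Pawns from the owner's location out to MeleeAttackRange.
; A hit actor with a BPC_Health component takes fixed damage through that component's TakeDamage.
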(event EventBeginPlay)

(event EventTick
  (params (DeltaSeconds :type Float%20%28single-precision%29)))

(fn UseMeleeAttack
  (bind _returnvalue (Components|GetOwner))
  (bind _returnvalue_2 (Transformation|GetActorLocation _returnvalue))
  (bind _look_direction (Class|BPICharacter|GetLookDirection(Message) _returnvalue))
  (bind _output_get (LocalVariables|SetLook%20Direction _look_direction))
  (bind (_outhit _returnvalue_3) (Class|KismetSystemLibrary|CapsuleTraceSingleforObjects _returnvalue_2 (+ (* _output_get (Variables|Default|GetMelee%20Attack%20Range)) _returnvalue_2) 1e+02 125.0 (Utilities|Array|MakeArray "ObjectTypeQuery3") false 0 "None" true))
  (if _returnvalue_3
    (Utilities|IsValid (Actor|GetComponentbyClass (.HitActor (Collision|BreakHitResult _outhit)) "/Game/Components/BPC_Health.BPC_Health_C")
      (:Is%20Valid
        (Default|TakeDamage (Actor|GetComponentbyClass (.HitActor (Collision|BreakHitResult _outhit)) "/Game/Components/BPC_Health.BPC_Health_C") 3e+01)))))