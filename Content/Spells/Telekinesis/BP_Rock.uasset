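; BP_Rock is a rock actor for the Telekinesis spell that deals damage when it hits something after being launched.
; On a sphere hit, it checks that its telekinesis object component is flagged as launched and that the other actor is not that component's owner.
; If that actor has a BPC_Health component, it applies fixed damage and clears the launched flag, so only the first such hit counts.
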(event OnComponentHit(Sphere)
  (params (HitComponent :type Primitive%20Component%20Object%20Reference) (OtherActor :type Actor%20Object%20Reference) (OtherComp :type Primitive%20Component%20Object%20Reference) (NormalImpulse :type Vector :default "0, 0, 0") (Hit :type Hit%20Result%20Structure%20%28by%20ref%29))
  (bind _returnvalue (Actor|GetComponentbyClass OtherActor "/Game/Components/BPC_Health.BPC_Health_C"))
  (bind _bpc_telekinesisobject (Variables|Default|GetBPC_TelekinesisObject))
  (if (and (Variables|/Game/Spells/Telekinesis/BPC_TelekinesisObject.BPC_TelekinesisObject_C|GetHas%20Been%20Launched _bpc_telekinesisobject) (not (== OtherActor (Components|GetOwner _bpc_telekinesisobject))))
    (Utilities|IsValid _returnvalue
      (:Is%20Valid
        (Default|TakeDamage _returnvalue 4e+01)
        (Variables|/Game/Spells/Telekinesis/BPC_TelekinesisObject.BPC_TelekinesisObject_C|SetHas%20Been%20Launched (Variables|Default|GetBPC_TelekinesisObject) false)))))

(event EventBeginPlay)

(event Collision|EventActorBeginOverlap
  (params (OtherActor :type Actor%20Object%20Reference)))

(event EventTick
  (params (DeltaSeconds :type Float%20%28single-precision%29)))

(fn ConstructionScript)