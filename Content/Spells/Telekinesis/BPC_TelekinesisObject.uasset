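; Component that lets the player hold, pull, push and launch an object with telekinesis.
; While the pawn's telekinesis component is active, Tick disables gravity and moves the owner toward the look point at a stored distance from the center-mass indicator.
; Pull and push offset the owner along the look direction and refresh that distance.
; Gravity and launch impulse target the first BP_Rock found at BeginPlay, rather than the owner.
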(event Custom|Push%20From%20Holder
  (bind _returnvalue (Components|GetOwner))
  (CallFunction|UpdateLookDirection)
  (Transformation|SetActorLocation _returnvalue (+ (* (Variables|Default|GetLook%20Direction) (Variables|Default|GetPush%20Force)) (Transformation|GetActorLocation _returnvalue)) true false)
  (CallFunction|UpdateHoldertoObjectDistance))

(event Custom|Pull%20To%20Holder
  (bind _returnvalue (Components|GetOwner))
  (CallFunction|UpdateLookDirection)
  (Transformation|SetActorLocation _returnvalue (+ (* (* (Variables|Default|GetLook%20Direction) "-1.000000,-1.000000,-1.000000") (Variables|Default|GetPull%20Force)) (Transformation|GetActorLocation _returnvalue)) false false)
  (CallFunction|UpdateHoldertoObjectDistance))

(event Custom|Launch
  (CallFunction|UpdateLookDirection)
  (Physics|AddImpulse (Variables|/Game/Spells/Telekinesis/BP_Rock.BP_Rock_C|GetSphere (Variables|Default|GetObject)) (* (Variables|Default|GetLook%20Direction) (Variables|Default|GetLaunch%20Force)) "None" false)
  (Variables|Default|SetHas%20Been%20Launched true))

(event EventBeginPlay
  (Variables|Default|SetHolder (Game|Player|GetPlayerPawn 0))
  (bind _returnvalue (Actor|GetActorOfClass "/Game/Spells/Telekinesis/BP_Rock.BP_Rock_C"))
  (CallFunction|SetObject _returnvalue)
  (Variables|Default|SetTelekinesis%20User%20Component (Actor|GetComponentbyClass (Variables|Default|GetHolder) "/Game/Spells/Telekinesis/BPC_TelekinesisUser.BPC_TelekinesisUser_C"))
  (CallFunction|UpdateHoldertoObjectDistance))

(event EventTick
  (params (DeltaSeconds :type Float%20%28single-precision%29))
  (bind _object (Variables|Default|GetObject))
  (bind _sphere (Variables|/Game/Spells/Telekinesis/BP_Rock.BP_Rock_C|GetSphere _object))
  (if (Variables|/Game/Spells/Telekinesis/BPC_TelekinesisUser.BPC_TelekinesisUser_C|GetIs%20Using%20Telekinesis (Variables|Default|GetTelekinesis%20User%20Component))
    (Physics|SetEnableGravity _sphere false)
    (CallFunction|MovetoCenter)
    (else
      (Physics|SetEnableGravity _sphere true))))

(fn SetObject
  (params (New%20Object :type BP%20Rock%20Object%20Reference))
  (Variables|Default|SetObject New%20Object))

(fn UpdateLookDirection
  (bind _look_direction (Class|BPICharacter|GetLookDirection(Message) (Variables|Default|GetHolder)))
  (Variables|Default|SetLook%20Direction _look_direction))

(fn MovetoCenter
  (bind _returnvalue (Components|GetOwner))
  (bind _output_get (LocalVariables|SetHolder%20Look%20Location (Transformation|GetWorldLocation (Actor|GetComponentbyClass (Variables|Default|GetHolder) "/Game/Components/BPC_CenterMassIndicator.BPC_CenterMassIndicator_C"))))
  (CallFunction|UpdateLookDirection)
  (Transformation|SetActorLocation _returnvalue (Class|VectorFunctionLibrary|GetPointatLookDistance (Variables|Default|GetLook%20Direction) _output_get (Variables|Default|GetHolder%20to%20Object%20Distance) (Transformation|GetActorLocation _returnvalue)) true false))

(fn UpdateHoldertoObjectDistance
  (Variables|Default|SetHolder%20to%20Object%20Distance (Class|VectorFunctionLibrary|GetDistance (Transformation|GetActorLocation (Components|GetOwner)) (Transformation|GetWorldLocation (Actor|GetComponentbyClass (Variables|Default|GetHolder) "/Game/Components/BPC_CenterMassIndicator.BPC_CenterMassIndicator_C")))))