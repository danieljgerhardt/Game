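; Actor component for the telekinesis spell that lets its owner grab a rock and launch it.
; Enable sphere-traces physics bodies along the owner's interface-provided look direction, accepts only a BP_Rock, outlines it with an overlay material and hands it to the rock's telekinesis component.
; Disable clears the outline and calls Launch on that component, without checking that a rock is held.
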(event EventBeginPlay)

(event EventTick
  (params (DeltaSeconds :type Float%20%28single-precision%29)))

(fn DisableTelekinesis
  (bind _telekinesis_object (Variables|Default|GetTelekinesis%20Object))
  (Variables|Default|SetIs%20Using%20Telekinesis false)
  (Rendering|Material|SetOverlayMaterial (Variables|/Game/Spells/Telekinesis/BP_Rock.BP_Rock_C|GetSphere _telekinesis_object) 0 :!class /Script/Engine.MeshComponent)
  (Default|Launch (Variables|/Game/Spells/Telekinesis/BP_Rock.BP_Rock_C|GetBPC_TelekinesisObject _telekinesis_object)))

(fn EnableTelekinesis
  (bind _returnvalue (Components|GetOwner))
  (bind _returnvalue_2 (Transformation|GetActorLocation _returnvalue))
  (bind _look_direction (Class|BPICharacter|GetLookDirection(Message) _returnvalue))
  (bind (_outhit _returnvalue_3) (Collision|SphereTraceForObjects _returnvalue_2 (+ (* _look_direction 1e+04) _returnvalue_2) 5e+02 (Utilities|Array|MakeArray "ObjectTypeQuery4") false 0 "None"))
  (if _returnvalue_3
    (bind _asbp_rock (Utilities|Casting|CastToBP_Rock (.HitActor (Collision|BreakHitResult _outhit))))
    (Rendering|Material|SetOverlayMaterial (Variables|/Game/Spells/Telekinesis/BP_Rock.BP_Rock_C|GetSphere _asbp_rock) "/Game/Spells/Telekinesis/M_Outline.M_Outline" :!class /Script/Engine.MeshComponent)
    (Variables|Default|SetIs%20Using%20Telekinesis true)
    (bind _output_get (Variables|Default|SetTelekinesis%20Object _asbp_rock))
    (Default|SetObject (Variables|/Game/Spells/Telekinesis/BP_Rock.BP_Rock_C|GetBPC_TelekinesisObject _output_get) _asbp_rock)))