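; Blueball spell projectile that launches along a look direction, homes in on a target and damages overlapped actors with BPC_Health.
; On cast, it targets the player if the nearest BP_BaseEnemy is closer than the player, otherwise that enemy.
; Tick slerps velocity toward slightly above the target, pausing for uncontrolled enemies.
; Any overlap deactivates movement, destroys the sphere and activates particles.
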(event EventBeginPlay)

(event EventCreateParticles
  (Components|Activation|Deactivate (Variables|Default|GetProjectileMovement))
  (Components|DestroyComponent (Variables|Default|GetSphere))
  (Components|Activation|Activate (Variables|Default|GetParticleSystem) false))

(event EventTick
  (params (DeltaSeconds :type Float%20%28single-precision%29))
  (CallFunction|UpdateVelocity))

(event EventCastSpell
  (params (Look%20Direction :type Vector :default "0, 0, 0"))
  (Game|Components|ProjectileMovement|SetVelocityinLocalSpace (Variables|Default|GetProjectileMovement) (* Look%20Direction (Variables|Default|GetShoot%20Speed)))
  (CallFunction|SetupTarget))

(event Collision|EventActorBeginOverlap
  (params (OtherActor :type Actor%20Object%20Reference))
  (bind _returnvalue (Actor|GetComponentbyClass OtherActor "/Game/Components/BPC_Health.BPC_Health_C"))
  (CallFunction|CreateParticles)
  (Utilities|IsValid _returnvalue
    (:Is%20Valid
      (Default|TakeDamage _returnvalue (Variables|Default|GetDamage%20Amount)))))

(fn ConstructionScript)

(fn FindTargets
  (return 0))

(fn SetupTarget
  (bind _returnvalue (Transformation|GetActorLocation))
  (bind _outactors (Actor|GetAllActorsOfClass "/Game/NPCs/Enemies/BP_BaseEnemy.BP_BaseEnemy_C"))
  (if (<= (Utilities|Array|Length _outactors) 0)
    (return)
    (else
      (for _array_element _outactors
        (if (< (Math|Vector|VectorLength (- (Transformation|GetActorLocation _array_element) _returnvalue)) (LocalVariables|GetMin%20Distance))
          (LocalVariables|SetMin%20Distance (Math|Vector|VectorLength (- (Transformation|GetActorLocation _array_element) _returnvalue)))
          (bind _output_get (LocalVariables|SetClosest%20Enemy _array_element))))
      (if (< (LocalVariables|GetMin%20Distance) (Math|Vector|VectorLength (- (Transformation|GetActorLocation (Game|Player|GetPlayerPawn 0)) _returnvalue)))
        (Variables|Default|SetTarget (Game|Player|GetPlayerPawn 0))
        (else
          (Variables|Default|SetTarget _output_get)
          (Variables|Default|SetIs%20Target%20Enemy true))))))

(fn UpdateVelocity
  (bind _target (Variables|Default|GetTarget))
  (Utilities|IsValid _target
    (:Is%20Valid
      (if (not (and (Variables|Default|GetIs%20Target%20Enemy) (not (Class|Pawn|IsPawnControlled (Variables|Default|GetTarget)))))
        (Game|Components|ProjectileMovement|SetVelocityinLocalSpace (Variables|Default|GetProjectileMovement) (Class|KismetMathLibrary|VectorSlerpVectortoDirection (Variables|/Script/Engine.MovementComponent|GetVelocity (Variables|Default|GetProjectileMovement)) (* (Math|Vector|Normalize (- (+ (Transformation|GetActorLocation _target) "0.000000,0.000000,75.000000") (Transformation|GetActorLocation))) (Variables|Default|GetShoot%20Speed)) 0.1))))))