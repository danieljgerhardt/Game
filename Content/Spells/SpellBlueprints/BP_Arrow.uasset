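; BP_Arrow is a physics-driven arrow projectile that damages Characters it overlaps.
; On overlap it attaches to the Character's skeletal mesh, stops simulating physics and ignores that actor when moving.
; It passes a damage amount, fetched from its owner by interface message, to the target's BPC_Health component.
; Tick destroys the actor whenever the arrow's physics velocity drops to near zero.
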(event OnComponentBeginOverlap(Arrow)
  (params (OverlappedComponent :type Primitive%20Component%20Object%20Reference) (OtherActor :type Actor%20Object%20Reference) (OtherComp :type Primitive%20Component%20Object%20Reference) (OtherBodyIndex :type Integer) (bFromSweep :type Boolean) (SweepResult :type Hit%20Result%20Structure%20%28by%20ref%29))
  (bind _arrow (Variables|Default|GetArrow))
  (Utilities|Casting|CastToCharacter OtherActor)
  (Transformation|AttachComponentToComponent (Variables|Default|GetArrow) (Actor|GetComponentbyClass OtherActor "/Script/Engine.SkeletalMeshComponent") "None" "KeepWorld" "KeepWorld" "KeepWorld" true)
  (Physics|SetSimulatePhysics _arrow false)
  (Collision|IgnoreActorwhenMoving _arrow OtherActor true)
  (bind _damage_amount (Class|BPISpell|GetDamageAmount(Message) (Components|GetOwner)))
  (Default|TakeDamage (Actor|GetComponentbyClass OtherActor "/Game/Components/BPC_Health.BPC_Health_C") _damage_amount))

(event EventBeginPlay)

(event EventTick
  (params (DeltaSeconds :type Float%20%28single-precision%29))
  (bind _returnvalue (Physics|GetPhysicsLinearVelocity (Variables|Default|GetArrow) "None"))
  (if (<= (Math|Vector|VectorLength _returnvalue) 0.1)
    (Actor|DestroyActor)))

(fn ConstructionScript)