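; BP_Knife is a spell projectile that the player steers from a camera riding along with the knife.
; Casting freezes character movement, then each tick moves the first-person camera to the knife's camera point and drives velocity and knife rotation from the camera's view.
; On overlap it restores walking and camera position, stops ticking, swaps knife and ribbon trail for impact particles, and damages any BPC_Health component.
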(event EventBeginPlay
  (Collision|IgnoreActorwhenMoving (Variables|Default|GetKnife) (Components|GetOwner) true))

(event EventCreateParticles
  (Components|Activation|Deactivate (Variables|Default|GetProjectileMovement))
  (Components|DestroyComponent (Variables|Default|GetKnife))
  (Components|Activation|Activate (Variables|Default|GetParticleSystem) false)
  (Components|Activation|SetActive (Variables|Default|GetNS_RibbonTrail) false false))

(event EventTick
  (params (DeltaSeconds :type Float%20%28single-precision%29))
  (CallFunction|UpdateCamera)
  (CallFunction|UpdateVelocity))

(event EventCastSpell
  (params (Look%20Direction :type Vector :default "0, 0, 0"))
  (bind _asbp_first_person_character (Utilities|Casting|CastToBP_FirstPersonCharacter (Game|Player|GetPlayerPawn 0)))
  (Variables|Default|SetFirst%20Person%20Character _asbp_first_person_character)
  (CallFunction|DisableMovement))

(event Collision|EventActorBeginOverlap
  (params (OtherActor :type Actor%20Object%20Reference))
  (bind _returnvalue (Actor|GetComponentbyClass OtherActor "/Game/Components/BPC_Health.BPC_Health_C"))
  (CallFunction|EnableMovement)
  (CallFunction|CreateParticles)
  (Utilities|IsValid _returnvalue
    (:Is%20Valid
      (Default|TakeDamage _returnvalue (Variables|Default|GetDamage%20Amount)))))

(fn ConstructionScript)

(fn UpdateCamera
  (Transformation|SetWorldLocation (Variables|/Game/FirstPerson/Blueprints/BP_FirstPersonCharacter.BP_FirstPersonCharacter_C|GetFirstPersonCamera (Variables|Default|GetFirst%20Person%20Character)) (.location (Transformation|GetWorldTransform (Variables|Default|GetCamera%20Location))) true false))

(fn DisableMovement
  (Pawn|Components|CharacterMovement|SetMovementMode (Variables|/Script/Engine.Character|GetCharacterMovement (Variables|Default|GetFirst%20Person%20Character)) "MOVE_None" 0))

(fn EnableMovement
  (bind _first_person_character (Variables|Default|GetFirst%20Person%20Character))
  (Pawn|Components|CharacterMovement|SetMovementMode (Variables|/Script/Engine.Character|GetCharacterMovement _first_person_character) "MOVE_Walking" 0)
  (Actor|Tick|SetActorTickEnabled false)
  (Transformation|SetRelativeLocation (Variables|/Game/FirstPerson/Blueprints/BP_FirstPersonCharacter.BP_FirstPersonCharacter_C|GetFirstPersonCamera _first_person_character) "0.000000,6.543846,165.368983" false true))

(fn UpdateVelocity
  (bind _first_person_character (Variables|Default|GetFirst%20Person%20Character))
  (bind _firstpersoncamera (Variables|/Game/FirstPerson/Blueprints/BP_FirstPersonCharacter.BP_FirstPersonCharacter_C|GetFirstPersonCamera _first_person_character))
  (Game|Components|ProjectileMovement|SetVelocityinLocalSpace (Variables|Default|GetProjectileMovement) (* (Math|Vector|GetForwardVector _firstpersoncamera) (Variables|Default|GetShoot%20Speed)))
  (Transformation|SetWorldRotation (Variables|Default|GetKnife) (Transformation|GetWorldRotation _firstpersoncamera) false false))