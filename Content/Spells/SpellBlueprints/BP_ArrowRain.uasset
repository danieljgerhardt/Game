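; Arrow Rain spell that spawns rows of BP_Arrow actors in the air over an area extending along the cast's look direction.
; CastSpell loops on a short delay, with CallSAR placing each successive row farther from the spell actor along the flattened look direction.
; SpawnArrowRow spreads arrows perpendicular to that direction at absolute world height SpawnHeight, adding a forward offset and randomized position and rotation.
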(event EventBeginPlay)

(event EventCreateParticles)

(event EventTick
  (params (DeltaSeconds :type Float%20%28single-precision%29)))

(event EventCastSpell
  (params (Look%20Direction :type Vector :default "0, 0, 0"))
  (bind _current_iteration (Variables|Default|GetCurrent%20Iteration))
  (CallFunction|CallSAR (Variables|Default|GetCurrent%20Iteration) Look%20Direction :!label _label)
  (Math|Integer|IncrementInt _current_iteration
    (:%20%20
      (if (< _current_iteration (Variables|Default|GetNumber%20of%20Rows))
        (Utilities|FlowControl|Delay 0.2)
        (goto _label)))))

(event Collision|EventActorBeginOverlap
  (params (OtherActor :type Actor%20Object%20Reference)))

(fn ConstructionScript)

(fn FindTargets
  (return 0))

(fn SpawnArrowRow
  (params (Row%20Location :type Vector) (Spawn%20Direction :type Vector) (Look%20Direction :type Vector))
  (bind _half_arrow_count (Variables|Default|GetHalf%20Arrow%20Count))
  (for _index (range (* _half_arrow_count -1) _half_arrow_count)
    (Game|SpawnActorfromClass "/Game/Spells/SpellBlueprints/BP_Arrow.BP_Arrow_C" (Math|Transform|MakeTransform (+ (* (+ (- Row%20Location (* (/ (* _index (Variables|Default|GetSpawn%20Area%20Half%20Width)) _half_arrow_count) Spawn%20Direction)) (* Look%20Direction (Variables|Default|GetSpawn%20Offset))) "1.000000,1.000000,0.000000") (Math|Vector|MakeVector 0.0 0.0 (Variables|Default|GetSpawn%20Height)) (* (Math|Random|RandomUnitVector) (Variables|Default|GetRandom%20Perturb%20Range)) (Math|Vector|MakeVector 0.0 0.0 (* (Math|Random|RandomFloat) 2e+02))) (Math|Rotator|MakeRotator (* (Math|Random|RandomFloat) 4.0) (* (Math|Random|RandomFloat) 4.0) (* (Math|Random|RandomFloat) 3.6e+02))) "Undefined" "MultiplyWithRoot" self 0)))

(fn CallSAR
  (params (Index :type Integer) (Look%20Direction :type Vector))
  (CallFunction|SpawnArrowRow (+ (* (* (/ Index (Variables|Default|GetNumber%20of%20Rows)) (Variables|Default|GetSpawn%20Area%20Length)) (Math|Vector|Normalize (* Look%20Direction "1.000000,1.000000,0.000000"))) (Transformation|GetActorLocation)) (Math|Vector|Normalize (* (Math|Vector|RotateVectorAroundAxis Look%20Direction 9e+01 "0.000000,0.000000,1.000000") "1.000000,1.000000,0.000000")) Look%20Direction))