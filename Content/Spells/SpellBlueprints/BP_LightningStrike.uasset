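; Lightning strike spell actor that damages pawns around the point player 0 is looking at.
; On BeginPlay it line-traces on Visibility from just above that pawn's location along its look direction, up to MaxDistance.
; On a hit it deals fixed damage through BPC_Health to all pawns within DamageRange of the impact, then moves the Zap effect there and activates it.
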(event EventBeginPlay
  (bind _returnvalue (Game|Player|GetPlayerPawn 0))
  (bind _zap (Variables|Default|GetZap))
  (bind _returnvalue_2 (Transformation|GetActorLocation _returnvalue))
  (bind _returnvalue_3 (+ _returnvalue_2 "0.000000,0.000000,65.000000"))
  (|CallParentFunction)
  (bind _look_direction (Class|BPICharacter|GetLookDirection(Message) _returnvalue))
  (bind (_outhit _returnvalue_4) (Collision|LineTraceByChannel _returnvalue_3 (+ _returnvalue_3 (* _look_direction (Variables|Default|GetMax%20Distance))) "TraceTypeQuery1" false 0 "None"))
  (if _returnvalue_4
    (bind _out_pawns_in_range (CallFunction|GetAllPawnsinRange (.Location (Collision|BreakHitResult _outhit)) (Variables|Default|GetDamage%20Range) (Variables|Default|GetActors%20in%20Range)))
    (for _array_element _out_pawns_in_range
      (Default|TakeDamage (Actor|GetComponentbyClass _array_element "/Game/Components/BPC_Health.BPC_Health_C") 5e+01))
    (Transformation|SetWorldLocation _zap (.Location (Collision|BreakHitResult _outhit)) false true)
    (Components|Activation|Activate _zap false)))

(event Collision|EventActorBeginOverlap
  (params (OtherActor :type Actor%20Object%20Reference))
  (|CallParentFunction OtherActor) ; This node is disabled and will not be called.\nDrag off pins to build functionality.
)

(event EventTick
  (params (DeltaSeconds :type Float%20%28single-precision%29))
  (|CallParentFunction DeltaSeconds) ; This node is disabled and will not be called.\nDrag off pins to build functionality.
)

(fn ConstructionScript
  (|CallParentFunction))