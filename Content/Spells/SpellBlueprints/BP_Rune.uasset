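; BP_Rune is a spell that places a proximity rune on the surface hit by a line trace along the look direction.
; It marks the spot with a surface-aligned debug circle, moves and sizes its collision sphere there, and starts a duration timer.
; Either an overlap or timer expiry spawns a radius-scaled explosion, damages in-range pawns through BPC_Health, and destroys the actor.
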(event OnComponentBeginOverlap(SphereCollision)
  (params (OverlappedComponent :type Primitive%20Component%20Object%20Reference) (OtherActor :type Actor%20Object%20Reference) (OtherComp :type Primitive%20Component%20Object%20Reference) (OtherBodyIndex :type Integer) (bFromSweep :type Boolean) (SweepResult :type Hit%20Result%20Structure%20%28by%20ref%29))
  (bind _radius (Variables|Default|GetRadius))
  (bind _returnvalue (/ _radius 2e+01))
  (Effects|SpawnEmitteratLocation "/Game/StarterContent/Particles/P_Explosion.P_Explosion" (Variables|Default|GetRune%20Location) "0, 0, 0" (Math|Vector|MakeVector _returnvalue _returnvalue _returnvalue))
  (bind _out_pawns_in_range (CallFunction|GetAllPawnsinRange (Variables|Default|GetRune%20Location) (Variables|Default|GetRadius) (Variables|Default|GetPawns%20in%20Range)))
  (for _array_element _out_pawns_in_range
    (Utilities|IsValid (Actor|GetComponentbyClass _array_element "/Game/Components/BPC_Health.BPC_Health_C")
      (:Is%20Valid
        (Default|TakeDamage (Actor|GetComponentbyClass _array_element "/Game/Components/BPC_Health.BPC_Health_C") (Variables|Default|GetDamage%20Amount)))))
  (Actor|DestroyActor))

(event Custom|On%20Duration%20Finished
  (bind _radius (Variables|Default|GetRadius))
  (bind _returnvalue (/ _radius 2e+01))
  (Effects|SpawnEmitteratLocation "/Game/StarterContent/Particles/P_Explosion.P_Explosion" (Variables|Default|GetRune%20Location) "0, 0, 0" (Math|Vector|MakeVector _returnvalue _returnvalue _returnvalue))
  (bind _out_pawns_in_range (CallFunction|GetAllPawnsinRange (Variables|Default|GetRune%20Location) (Variables|Default|GetRadius) (Variables|Default|GetPawns%20in%20Range)))
  (for _array_element _out_pawns_in_range
    (Utilities|IsValid (Actor|GetComponentbyClass _array_element "/Game/Components/BPC_Health.BPC_Health_C")
      (:Is%20Valid
        (Default|TakeDamage (Actor|GetComponentbyClass _array_element "/Game/Components/BPC_Health.BPC_Health_C") (Variables|Default|GetDamage%20Amount)))))
  (Actor|DestroyActor))

(event EventBeginPlay
  (|CallParentFunction) ; This node is disabled and will not be called.\nDrag off pins to build functionality.
)

(event Collision|EventActorBeginOverlap
  (params (OtherActor :type Actor%20Object%20Reference))
  (|CallParentFunction OtherActor) ; This node is disabled and will not be called.\nDrag off pins to build functionality.
)

(event EventTick
  (params (DeltaSeconds :type Float%20%28single-precision%29))
  (|CallParentFunction DeltaSeconds))

(event EventCastSpell
  (params (Look%20Direction :type Vector :default "0, 0, 0"))
  (bind _returnvalue (Transformation|GetActorLocation))
  (bind _sphere_collision (Variables|Default|GetSphere%20Collision))
  (bind (_outhit _returnvalue_2) (Collision|LineTraceByChannel _returnvalue (+ _returnvalue (* Look%20Direction 8e+03)) "TraceTypeQuery1" false 0 "None"))
  (if _returnvalue_2
    (bind _output_get (Variables|Default|SetRune%20Location (.ImpactPoint (Collision|BreakHitResult _outhit))))
    (Rendering|Debug|DrawDebugCircle _output_get (Variables|Default|GetRadius) 12 "(R=1.000000,G=0.429049,B=0.558214,A=1.000000)" (Variables|Default|GetDuration) 15.0 (Math|Vector|CrossProduct (.ImpactNormal (Collision|BreakHitResult _outhit)) "0.000000,1.000000,0.000000") (Math|Vector|CrossProduct (Math|Vector|CrossProduct (.ImpactNormal (Collision|BreakHitResult _outhit)) "0.000000,1.000000,0.000000") (.ImpactNormal (Collision|BreakHitResult _outhit))))
    (Transformation|SetWorldLocation _sphere_collision _output_get false false)
    (Variables|/Script/Engine.PrimitiveComponent|SetbGenerateOverlapEvents _sphere_collision true)
    (Components|Sphere|SetSphereRadius _sphere_collision (Variables|Default|GetRadius) false)
    (Utilities|Time|SetTimerbyEvent (delegate Custom|On%20Duration%20Finished) (Variables|Default|GetDuration))))

(fn ConstructionScript
  (|CallParentFunction))