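; BP_Fireball is a fireball spell projectile that damages what it overlaps.
; CastSpell launches it along the look direction and starts the trail, while its sphere ignores the owner when moving.
; On overlap it shuts off trail and movement, destroys the sphere, fires an impact particle system and damages any BPC_Health on the other actor.
; FindTargets is an empty stub, and the actor never destroys itself here.
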(event EventBeginPlay
  (Collision|IgnoreActorwhenMoving (Variables|Default|GetSphere) (Components|GetOwner) true))

(event EventCreateParticles
  (Components|Activation|SetActive (Variables|Default|GetParticleTrail) false false)
  (Components|Activation|Deactivate (Variables|Default|GetProjectileMovement))
  (Components|DestroyComponent (Variables|Default|GetSphere))
  (Components|Activation|Activate (Variables|Default|GetParticleSystem) false))

(event EventTick
  (params (DeltaSeconds :type Float%20%28single-precision%29)))

(event EventCastSpell
  (params (Look%20Direction :type Vector :default "0, 0, 0"))
  (Game|Components|ProjectileMovement|SetVelocityinLocalSpace (Variables|Default|GetProjectileMovement) (* Look%20Direction (Variables|Default|GetShoot%20Speed)))
  (Components|Activation|Activate (Variables|Default|GetParticleTrail) false))

(event Collision|EventActorBeginOverlap
  (params (OtherActor :type Actor%20Object%20Reference))
  (bind _returnvalue (Actor|GetComponentbyClass OtherActor "/Game/Components/BPC_Health.BPC_Health_C"))
  (CallFunction|CreateParticles)
  (Utilities|IsValid _returnvalue
    (:Is%20Valid
      (Default|TakeDamage _returnvalue (Variables|Default|GetDamage%20Amount)))))

(fn ConstructionScript)

(fn FindTargets
  (return 0))