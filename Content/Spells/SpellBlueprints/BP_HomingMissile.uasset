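; Homing missile spell projectile that launches along the cast direction and seeks an enemy or player's center-mass indicator.
; SetupTarget infers the side by proximity at cast, targeting the player if the nearest collidable enemy is closer than the player, otherwise that enemy.
; Tick aligns rotation to velocity and retargets when an enemy target loses capsule collision.
; Non-owner overlaps stop movement, switch trail to impact particles and apply BPC_Health damage.
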(event EventBeginPlay
  (Collision|IgnoreActorwhenMoving (Variables|Default|GetSphere) (Components|GetOwner) true))

(event EventCreateParticles
  (Components|Activation|Deactivate (Variables|Default|GetProjectileMovement))
  (Components|DestroyComponent (Variables|Default|GetSphere))
  (Components|Activation|Activate (Variables|Default|GetParticleSystem) false)
  (Components|Activation|SetActive (Variables|Default|GetNS_RibbonTrail) false false))

(event EventTick
  (params (DeltaSeconds :type Float%20%28single-precision%29))
  (bind _target (Variables|Default|GetTarget))
  (Transformation|SetActorRotation (Math|Rotator|FindLookatRotation (Math|Vector|MakeVector 0.0 0.0 0.0) (Transformation|GetVelocity)))
  (Utilities|IsValid _target
    (:Is%20Valid
      (bind _asbp_base_enemy (Utilities|Casting|CastToBP_BaseEnemy _target))
      (if (not (Class|PrimitiveComponent|IsCollisionEnabled (Variables|/Script/Engine.Character|GetCapsuleComponent _asbp_base_enemy)))
        (bind _scene_component (CallFunction|SetupTarget true))
        (Variables|/Script/Engine.ProjectileMovementComponent|SetHomingTargetComponent (Variables|Default|GetProjectileMovement) _scene_component)))))

(event EventCastSpell
  (params (Look%20Direction :type Vector :default "0, 0, 0"))
  (Game|Components|ProjectileMovement|SetVelocityinLocalSpace (Variables|Default|GetProjectileMovement) (* Look%20Direction (Variables|Default|GetShoot%20Speed)))
  (bind _scene_component (CallFunction|SetupTarget false))
  (Variables|/Script/Engine.ProjectileMovementComponent|SetHomingTargetComponent (Variables|Default|GetProjectileMovement) _scene_component)
  (Components|Activation|Activate (Variables|Default|GetNS_RibbonTrail) false))

(event Collision|EventActorBeginOverlap
  (params (OtherActor :type Actor%20Object%20Reference))
  (bind _returnvalue (Actor|GetComponentbyClass "/Game/Components/BPC_Health.BPC_Health_C"))
  (if (!= OtherActor (Components|GetOwner))
    (CallFunction|CreateParticles)
    (Utilities|IsValid _returnvalue
      (:Is%20Valid
        (Default|TakeDamage _returnvalue (Variables|Default|GetDamage%20Amount))))))

(fn ConstructionScript)

(fn FindTargets
  (return 0))

(fn SetupTarget
  (params (isPlayer :type Boolean))
  (bind _returnvalue (Transformation|GetActorLocation))
  (bind _outactors (Actor|GetAllActorsOfClass "/Game/NPCs/Enemies/BP_BaseEnemy.BP_BaseEnemy_C"))
  (if (<= (Utilities|Array|Length _outactors) 0)
    (return 0)
    (else
      (for _array_element _outactors
        (if (Class|PrimitiveComponent|IsCollisionEnabled (Variables|/Script/Engine.Character|GetCapsuleComponent _array_element))
          (if (< (Math|Vector|VectorLength (- (Transformation|GetActorLocation _array_element) _returnvalue)) (LocalVariables|GetMin%20Distance))
            (LocalVariables|SetMin%20Distance (Math|Vector|VectorLength (- (Transformation|GetActorLocation _array_element) _returnvalue)))
            (bind _output_get (LocalVariables|SetClosest%20Enemy _array_element)))))
      (if isPlayer
        _
        (elif (< (LocalVariables|GetMin%20Distance) (Math|Vector|VectorLength (- (Transformation|GetActorLocation (Game|Player|GetPlayerPawn 0)) _returnvalue)))
          (bind _output_get_2 (Variables|Default|SetTarget (Game|Player|GetPlayerPawn 0)))
          (return (Actor|GetComponentbyClass _output_get_2 "/Game/Components/BPC_CenterMassIndicator.BPC_CenterMassIndicator_C"))
          (else
            _)))
      (bind _output_get_3 (Variables|Default|SetTarget _output_get))
      (Utilities|IsValid _output_get_3
        (:Is%20Valid
          (Variables|Default|SetIs%20Target%20Enemy true)
          (return (Actor|GetComponentbyClass _output_get_3 "/Game/Components/BPC_CenterMassIndicator.BPC_CenterMassIndicator_C")))))))