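; Impact spell projectile that spins as it flies along the cast direction, trailing particles.
; Overlapping an enemy ragdolls and launches it, shuts down the projectile's movement and visuals, then, given a health component, deals damage, restoring the enemy and destroying itself after a delay.
; Other overlaps line-trace along velocity and reflect it off surfaces whose normal is not predominantly vertical, bouncing off walls.
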(event EventBeginPlay
  (bind _returnvalue (Components|GetOwner))
  (|CallParentFunction)
  (Collision|IgnoreActorwhenMoving (Variables|Default|GetStaticMesh) _returnvalue true)
  (Collision|IgnoreActorwhenMoving (Actor|GetComponentbyClass _returnvalue "/Script/Engine.CapsuleComponent") self true))

(event EventCreateParticles
  (Components|Activation|SetActive (Variables|Default|GetParticleTrail) false false)
  (Components|Activation|Deactivate (Variables|Default|GetProjectileMovement))
  (Components|DestroyComponent (Variables|Default|GetStaticMesh)))

(event EventTick
  (params (DeltaSeconds :type Float%20%28single-precision%29))
  (|CallParentFunction DeltaSeconds)
  (Transformation|SetActorRotation (Math|Rotator|CombineRotators (Transformation|GetActorRotation) "0.000000,20.000000,0.000000")))

(event EventCastSpell
  (params (Look%20Direction :type Vector :default "0, 0, 0"))
  (Game|Components|ProjectileMovement|SetVelocityinLocalSpace (Variables|Default|GetProjectileMovement) (* Look%20Direction (Variables|Default|GetShoot%20Speed)))
  (Transformation|SetActorRotation "5.000000,0.000000,0.000000")
  (Components|Activation|Activate (Variables|Default|GetParticleTrail) false))

(event Collision|EventActorBeginOverlap
  (params (OtherActor :type Actor%20Object%20Reference))
  (bind _returnvalue (Transformation|GetVelocity))
  (bind _returnvalue_2 (Actor|GetComponentbyClass OtherActor "/Game/Components/BPC_Health.BPC_Health_C"))
  (bind _returnvalue_3 (Transformation|GetActorLocation))
  (bind _projectilemovement (Variables|Default|GetProjectileMovement))
  (bind _asbp_base_enemy (Utilities|Casting|CastToBP_BaseEnemy OtherActor)
    (:then
      (Default|ToggleRagdoll _asbp_base_enemy true)
      (Physics|AddImpulse (Variables|/Script/Engine.Character|GetMesh _asbp_base_enemy) (Math|Vector|MakeVector (* (.x _returnvalue) 5e+01) (* (.y _returnvalue) 5e+01) 5e+04) "None" false)
      (CallFunction|CreateParticles)
      (Utilities|IsValid _returnvalue_2
        (:Is%20Valid
          (Default|TakeDamage _returnvalue_2 (Variables|Default|GetDamage%20Amount))
          (Utilities|FlowControl|Delay 3.0)
          (Default|ToggleRagdoll _asbp_base_enemy false)
          (Actor|DestroyActor))))
    (:CastFailed
      (bind _outhit (Collision|LineTraceByChannel _returnvalue_3 (+ _returnvalue_3 (Variables|/Script/Engine.MovementComponent|GetVelocity _projectilemovement)) "TraceTypeQuery1" false 0 "None"))
      (if (not (== (Math|Float|Max(Float) (Math|Float|Absolute(Float) (.X (Math|Vector|BreakVector (.normal _outhit)))) (Math|Float|Absolute(Float) (.Y (Math|Vector|BreakVector (.normal _outhit)))) (Math|Float|Absolute(Float) (.Z (Math|Vector|BreakVector (.normal _outhit))))) (Math|Float|Absolute(Float) (.Z (Math|Vector|BreakVector (.normal _outhit))))))
        (Variables|/Script/Engine.MovementComponent|SetVelocity _projectilemovement (Math|Vector|GetReflectionVector (Variables|/Script/Engine.MovementComponent|GetVelocity _projectilemovement) (.normal _outhit)))))))

(fn ConstructionScript
  (|CallParentFunction))